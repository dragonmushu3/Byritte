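; BP_BBElectricPlug is an electric plug actor that recharges the player character's BabyEnergy while the player stands in its Box trigger.
; Box overlap begin and end events set an Overlapped flag for the player character.
; Tick runs a free-running five-second accumulator, independent of overlap, that on each cycle adds a fixed amount of energy and plays the BBCharge sound if the flag is set.
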(event OnComponentBeginOverlap(Box)
  (params (OverlappedComponent :type Primitive%20Component%20Object%20Reference) (OtherActor :type Actor%20Object%20Reference) (OtherComp :type Primitive%20Component%20Object%20Reference) (OtherBodyIndex :type Integer) (bFromSweep :type Boolean) (SweepResult :type Hit%20Result%20Structure%20%28by%20ref%29))
  (Utilities|Casting|CastToBP_PlayerCharacter OtherActor)
  (Variables|Default|SetOverlapped? true))

(event OnComponentEndOverlap(Box)
  (params (OverlappedComponent :type Primitive%20Component%20Object%20Reference) (OtherActor :type Actor%20Object%20Reference) (OtherComp :type Primitive%20Component%20Object%20Reference) (OtherBodyIndex :type Integer))
  (Utilities|Casting|CastToBP_PlayerCharacter OtherActor)
  (Variables|Default|SetOverlapped? false))

(event EventBeginPlay)

(event Collision|EventActorBeginOverlap
  (params (OtherActor :type Actor%20Object%20Reference)))

(event EventTick
  (params (DeltaSeconds :type Float%20%28single-precision%29))
  (Variables|Default|SetTime (+ DeltaSeconds (Variables|Default|GetTime)))
  (if (> (Variables|Default|GetTime) 5.0)
    (Variables|Default|SetTime 0.0)
    (bind _asbp_player_character (Utilities|Casting|CastToBP_PlayerCharacter (Game|GetPlayerCharacter 0)))
    (if (Variables|Default|GetOverlapped?)
      (Variables|/Game/byritte/Blueprints/BP_PlayerCharacter.BP_PlayerCharacter_C|SetBabyEnergy _asbp_player_character (+ (Variables|/Game/byritte/Blueprints/BP_PlayerCharacter.BP_PlayerCharacter_C|GetBabyEnergy _asbp_player_character) 5.0))
      (Audio|PlaySoundatLocation "/Game/byritte/Sound/BBCharge.BBCharge" (Transformation|GetWorldLocation (Variables|Default|GetDefaultSceneRoot)) "0, 0, 0" 1.0 1.0 0.0 0 0 0 0))))

(fn ConstructionScript)